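; Poison pit hazard that warns the player by sound and kills them on contact.
; Inside the trigger radius, Tick turns the negated marker-to-player distance, derived from trace endpoints, into a homing signal whose pitch rises on approach.
; A closer trigger re-activates a whoosh in a randomly delayed loop.
; Touching the poison plays a death sound and destroys the player after a delay, with overlaps filtered to the cached player capsule.
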(event `self.ReceiveTick`
  (params (DeltaSeconds :type "Float (single-precision)"))
  (bind _obj_playercast (`self.obj_PlayerCast`))
  (bind _poisonwarningsignal (`self.PoisonWarningSignal`))
  ;[0.5655 0.6802 0] Homing Signal
  (if (`self.b_InPoisonHazardProx`)
    (`/Engine/EditorBlueprintResources/StandardMacros.IsValid` _obj_playercast
      (:`Is Valid`
        (bind _outhit (`KismetSystemLibrary.LineTraceSingle` (`SceneComponent.K2_GetComponentLocation` (`self.PoisonMarker`)) (+ (0.0 0.0 0.0) (* (`SceneComponent.K2_GetComponentLocation` (`Character.Mesh` _obj_playercast)) 1.0)) "TraceTypeQuery1"))
        (bind (_bblockinghit _binitialoverlap _time _distance _location _impactpoint _normal _impactnormal _physmat _hitactor _hitcomponent _hitbonename _bonename _hititem _elementindex _faceindex _tracestart _traceend) (`GameplayStatics.BreakHitResult` _outhit))
        (bind _output_get (set `self.fvar_PoisonCollisionPoint` (* (`KismetMathLibrary.GetPointDistanceToLine` _traceend _tracestart) -1.0)))
        (`ActorComponent.Activate` _poisonwarningsignal false)
        (`AudioComponent.SetPitchMultiplier` _poisonwarningsignal (+ (`KismetMathLibrary.NormalizeToRange` _output_get -1646.0 -400.0) 1.0))))))

(event `self.TriggerRadius.OnComponentBeginOverlap`
  (params (OverlappedComponent :type "PrimitiveComponent Object Reference") (OtherActor :type "Actor Object Reference") (OtherComp :type "PrimitiveComponent Object Reference") (OtherBodyIndex :type Integer) (bFromSweep :type Boolean) (SweepResult :type "HitResult Structure (by ref)"))
  (bind _obj_playercollision (`self.obj_PlayerCollision`))
  ;[0 1 0.5919] Exiting Poison Radius
  (`/Engine/EditorBlueprintResources/StandardMacros.IsValid` _obj_playercollision :!label _label
    (:`Is Valid`
      (if (== OtherComp _obj_playercollision)
        (`KismetSystemLibrary.PrintString` "INSIDE RADIUS" false true (struct :`R` 0.041959 :`G` 0.505208 :`A` 1.0) 5.0)
        (set `self.b_InPoisonHazardProx` true)))
    (:`Is Not Valid`
      (`self.SetUpPlayerCollision`
        (:`output`
          (goto _label))))))

(event `self.ReceiveBeginPlay`
  (`self.SetUpPlayerCollision`))

(event `self.TriggerRadius.OnComponentEndOverlap`
  (params (OverlappedComponent :type "PrimitiveComponent Object Reference") (OtherActor :type "Actor Object Reference") (OtherComp :type "PrimitiveComponent Object Reference") (OtherBodyIndex :type Integer))
  ;[0 1 0.5919] Exiting Poison Radius
  (if (== (`self.obj_PlayerCollision`) OtherComp)
    (`KismetSystemLibrary.PrintString` "LEFT RADIUS" false true (struct :`R` 0.505208 :`A` 1.0) 5.0)
    (set `self.b_InPoisonHazardProx` false)
    (`ActorComponent.Deactivate` (`self.PoisonWarningSignal`))))

(event `self.Collision_Poison.OnComponentBeginOverlap`
  (params (OverlappedComponent :type "PrimitiveComponent Object Reference") (OtherActor :type "Actor Object Reference") (OtherComp :type "PrimitiveComponent Object Reference") (OtherBodyIndex :type Integer) (bFromSweep :type Boolean) (SweepResult :type "HitResult Structure (by ref)"))
  (bind _obj_playercollision (`self.obj_PlayerCollision`))
  ;[1 0 0.008825] Death Sequence
  (`/Engine/EditorBlueprintResources/StandardMacros.IsValid` _obj_playercollision :!label _label_2
    (:`Is Valid`
      (if (== OtherComp _obj_playercollision)
        (`GameplayStatics.PlaySound2D` "/Game/Audio/SFX/PlayerAndEnemy/player_death_Cue.player_death_Cue" 1.0 1.0 0.0 null null)
        (`ActorComponent.Deactivate` (`self.WhooshSound`))
        (`KismetSystemLibrary.Delay` 0.5)
        (`self.K2_DestroyActor` (`self.obj_PlayerCast`))))
    (:`Is Not Valid`
      (`self.SetUpPlayerCollision`
        (:`output`
          (goto _label_2))))))

(event `self.WhooshTriggerB.OnComponentBeginOverlap`
  (params (OverlappedComponent :type "PrimitiveComponent Object Reference") (OtherActor :type "Actor Object Reference") (OtherComp :type "PrimitiveComponent Object Reference") (OtherBodyIndex :type Integer) (bFromSweep :type Boolean) (SweepResult :type "HitResult Structure (by ref)"))
  (bind _whooshsound (`self.WhooshSound`))
  (bind _obj_playercollision (`self.obj_PlayerCollision`))
  ;[1 0 0.194] Player Close to Poison Pit
  (`/Engine/EditorBlueprintResources/StandardMacros.IsValid` _obj_playercollision :!label _label_3
    (:`Is Valid`
      (if (== OtherComp _obj_playercollision)
        (set `self.b_WhooshClose` true)
        (if (`self.b_WhooshClose`) :!label _label_4
          (`ActorComponent.Activate` _whooshsound false)
          (`KismetSystemLibrary.Delay` (`KismetMathLibrary.RandomFloatInRange` 0.0 0.05))
          (goto _label_4)
          (else
            (`ActorComponent.Deactivate` _whooshsound)))))
    (:`Is Not Valid`
      (`self.SetUpPlayerCollision`
        (:`output`
          (goto _label_3))))))

(event `self.WhooshTriggerB.OnComponentEndOverlap`
  (params (OverlappedComponent :type "PrimitiveComponent Object Reference") (OtherActor :type "Actor Object Reference") (OtherComp :type "PrimitiveComponent Object Reference") (OtherBodyIndex :type Integer))
  ;[1 0 0.194] Player Close to Poison Pit
  (if (== (`self.obj_PlayerCollision`) OtherComp)
    (set `self.b_WhooshClose` false)))

(fn `UserConstructionScript`)