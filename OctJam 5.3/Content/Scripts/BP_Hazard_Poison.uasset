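; Poison pit hazard that warns the player by sound as they approach and reloads Level3_PATCH when their capsule touches the poison.
; Inside the outer radius, Tick measures from the pit's center marker to the player's mesh, raising the warning signal's pitch as distance shrinks.
; An inner trigger replays a whoosh on a short delay loop while overlapped, without checking which actor entered.
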(event `self.TriggerRadius.OnComponentBeginOverlap`
  (params (OverlappedComponent :type "PrimitiveComponent Object Reference") (OtherActor :type "Actor Object Reference") (OtherComp :type "PrimitiveComponent Object Reference") (OtherBodyIndex :type Integer) (bFromSweep :type Boolean) (SweepResult :type "HitResult Structure (by ref)"))
  ;[1 0 0.99] What to do when player enters or exits the Poison's radius
  (bind _asbp_main_character (cast `/Game/OctJam/Blueprints/Characters/BP_MainCharacter` (`GameplayStatics.GetPlayerCharacter` 0)))
  (if (== OtherComp (`Character.CapsuleComponent` _asbp_main_character))
    (`KismetSystemLibrary.PrintString` "INSIDE RADIUS" false true (struct :`R` 0.041959 :`G` 0.505208 :`A` 1.0) 5.0)
    (set `self.b_InPoisHazardProx` true)))

(event `self.TriggerRadius.OnComponentEndOverlap`
  (params (OverlappedComponent :type "PrimitiveComponent Object Reference") (OtherActor :type "Actor Object Reference") (OtherComp :type "PrimitiveComponent Object Reference") (OtherBodyIndex :type Integer))
  ;[1 0 0.99] What to do when player enters or exits the Poison's radius
  (if (== (`Character.CapsuleComponent` (stale `self.TriggerRadius.OnComponentBeginOverlap` _asbp_main_character)) OtherComp)
    (`KismetSystemLibrary.PrintString` "LEFT RADIUS" false true (struct :`R` 0.505208 :`A` 1.0) 5.0)
    (set `self.b_InPoisHazardProx` false)
    (`ActorComponent.Deactivate` (`self.PoisonWarningSignal`))))

(event `self.ReceiveTick`
  (params (DeltaSeconds :type "Float (single-precision)"))
  (bind _poisonwarningsignal (`self.PoisonWarningSignal`))
  ;[1 0 0.99] Homing Signal
  (if (`self.b_InPoisHazardProx`)
    (bind _asbp_main_character (cast `/Game/OctJam/Blueprints/Characters/BP_MainCharacter` (`GameplayStatics.GetPlayerCharacter` 0)))
    (bind _outhit (`KismetSystemLibrary.LineTraceSingle` (`SceneComponent.K2_GetComponentLocation` (`self.PoisonMarker`)) (+ (0.0 0.0 0.0) (* (`SceneComponent.K2_GetComponentLocation` (`Character.Mesh` _asbp_main_character)) 1.0)) "TraceTypeQuery1"))
    (bind (_bblockinghit _binitialoverlap _time _distance _location _impactpoint _normal _impactnormal _physmat _hitactor _hitcomponent _hitbonename _bonename _hititem _elementindex _faceindex _tracestart _traceend) (`GameplayStatics.BreakHitResult` _outhit))
    (bind _returnvalue (`KismetMathLibrary.GetPointDistanceToLine` _traceend _tracestart))
    (`KismetSystemLibrary.PrintString` (`KismetStringLibrary.Conv_DoubleToString` _returnvalue) false)
    (bind _output_get (set `self.fvar_PoisonCollisionPoint` (* _returnvalue -1.0)))
    (`ActorComponent.Activate` _poisonwarningsignal false)
    (`AudioComponent.SetPitchMultiplier` _poisonwarningsignal (+ (`KismetMathLibrary.NormalizeToRange` _output_get -1646.0 -400.0) 1.0))))

(event `self.WhooshTrigger.OnComponentBeginOverlap`
  (params (OverlappedComponent :type "PrimitiveComponent Object Reference") (OtherActor :type "Actor Object Reference") (OtherComp :type "PrimitiveComponent Object Reference") (OtherBodyIndex :type Integer) (bFromSweep :type Boolean) (SweepResult :type "HitResult Structure (by ref)"))
  ;[0 1 0.1213] Whoosh Sound when player is super close to poison pit
  (set `self.b_WhooshClose` true)
  (if (`self.b_WhooshClose`) :!label _label
    (`ActorComponent.Activate` (`self.WhooshSound`) false)
    (`KismetSystemLibrary.Delay` 0.2)
    (goto _label)))

(event `self.WhooshTrigger.OnComponentEndOverlap`
  (params (OverlappedComponent :type "PrimitiveComponent Object Reference") (OtherActor :type "Actor Object Reference") (OtherComp :type "PrimitiveComponent Object Reference") (OtherBodyIndex :type Integer))
  ;[0 1 0.1213] Whoosh Sound when player is super close to poison pit
  (`ActorComponent.Deactivate` (`self.WhooshSound`))
  (set `self.b_WhooshClose` false))

(event `self.Collision_Poison.OnComponentBeginOverlap`
  (params (OverlappedComponent :type "PrimitiveComponent Object Reference") (OtherActor :type "Actor Object Reference") (OtherComp :type "PrimitiveComponent Object Reference") (OtherBodyIndex :type Integer) (bFromSweep :type Boolean) (SweepResult :type "HitResult Structure (by ref)"))
  ;[0 0.3615 1] Poison Damage
  (bind _asbp_main_character (cast `/Game/OctJam/Blueprints/Characters/BP_MainCharacter` (`GameplayStatics.GetPlayerCharacter` 0)))
  (`KismetSystemLibrary.PrintString` "cast success" false true (struct :`G` 0.057742 :`B` 1.0 :`A` 1.0))
  (if (== (`Character.CapsuleComponent` _asbp_main_character) OtherComp)
    (`KismetSystemLibrary.PrintString` "Poisoned" true true (struct :`R` 1.0 :`B` 0.018158 :`A` 1.0) 5.0) ; Poison functions called here if needed
    (`GameplayStatics.OpenLevel` "Level3_PATCH") ; Restart level for player
  ))

(event `self.Collision_Poison.OnComponentEndOverlap`
  (params (OverlappedComponent :type "PrimitiveComponent Object Reference") (OtherActor :type "Actor Object Reference") (OtherComp :type "PrimitiveComponent Object Reference") (OtherBodyIndex :type Integer))
  ;[0 0.3615 1] Poison Damage
  ;;[0 0 0] What happens when player leaves poison pit (not currently planned)
)

(fn `UserConstructionScript`)