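; BP_ItemB is a collectible memory item that beeps while the player is nearby and disappears with a sound on touch, flagging itself collected.
; Trigger overlaps toggle the zone flag; Tick traces to the player, stores a negated distance and activates the beeper, though distance-based pitch is disconnected.
; A dialogue radius shows examine indicators, and GetObj sends description data to the pawn.
; Dialogue, counter and level-advance functions are defined but uncalled here.
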(event `self.DialogueRadius.OnComponentBeginOverlap`
  (params (OverlappedComponent :type "PrimitiveComponent Object Reference") (OtherActor :type "Actor Object Reference") (OtherComp :type "PrimitiveComponent Object Reference") (OtherBodyIndex :type Integer) (bFromSweep :type Boolean) (SweepResult :type "HitResult Structure (by ref)"))
  (`self.ShowExamineIndicator` OverlappedComponent OtherActor))

(event `/Game/OctJam/Blueprints/BPI_EnvInteraction.GetObj`
  (bind _returnvalue (`GameplayStatics.GetPlayerPawn` 0))
  (message `/Game/OctJam/Blueprints/BPI_EnvInteraction.SendDT` _returnvalue (`self.DT_CurrItemDescDT`))
  (message `/Game/OctJam/Blueprints/BPI_Examine.ShowIndicator` _returnvalue))

(event `self.DialogueRadius.OnComponentEndOverlap`
  (params (OverlappedComponent :type "PrimitiveComponent Object Reference") (OtherActor :type "Actor Object Reference") (OtherComp :type "PrimitiveComponent Object Reference") (OtherBodyIndex :type Integer))
  (message `/Game/OctJam/Blueprints/BPI_Examine.RemoveIndicator` OtherActor))

(event `self.TriggerRadius.OnComponentBeginOverlap`
  (params (OverlappedComponent :type "PrimitiveComponent Object Reference") (OtherActor :type "Actor Object Reference") (OtherComp :type "PrimitiveComponent Object Reference") (OtherBodyIndex :type Integer) (bFromSweep :type Boolean) (SweepResult :type "HitResult Structure (by ref)"))
  (bind _asbp_main_character (cast `/Game/OctJam/Blueprints/Characters/BP_MainCharacter` (`GameplayStatics.GetPlayerCharacter` 0)))
  ;[1 1 1] What to do when player enters or exits the item's radius (MEMORY SOUND)
  (if (== OtherComp (`Character.CapsuleComponent` _asbp_main_character))
    (`KismetSystemLibrary.PrintString` "INSIDE RADIUS" false true (struct :`R` 0.041959 :`G` 0.505208 :`A` 1.0) 5.0)
    (set `self.b_InItemRadZone` true)))

(event `self.CollectItem.OnComponentBeginOverlap`
  (params (OverlappedComponent :type "PrimitiveComponent Object Reference") (OtherActor :type "Actor Object Reference") (OtherComp :type "PrimitiveComponent Object Reference") (OtherBodyIndex :type Integer) (bFromSweep :type Boolean) (SweepResult :type "HitResult Structure (by ref)"))
  ;[1 1 1] Item Collection
  (bind _asbp_main_character (cast `/Game/OctJam/Blueprints/Characters/BP_MainCharacter` (`GameplayStatics.GetPlayerCharacter` 0)))
  (if (== OtherComp (`Character.CapsuleComponent` _asbp_main_character))
    (`GameplayStatics.PlaySound2D` "/Game/Audio/SFX/Memory/collect_memory_Cue.collect_memory_Cue" 1.0 1.0 0.0 null null)
    (`self.K2_DestroyActor`)
    (set `self.b_Collected_ItemB` true)))

(event `self.TriggerRadius.OnComponentEndOverlap`
  (params (OverlappedComponent :type "PrimitiveComponent Object Reference") (OtherActor :type "Actor Object Reference") (OtherComp :type "PrimitiveComponent Object Reference") (OtherBodyIndex :type Integer))
  (bind _asbp_main_character (cast `/Game/OctJam/Blueprints/Characters/BP_MainCharacter` (`GameplayStatics.GetPlayerCharacter` 0)))
  ;[1 1 1] What to do when player enters or exits the item's radius (MEMORY SOUND)
  (if (== (`Character.CapsuleComponent` _asbp_main_character) OtherComp)
    (`KismetSystemLibrary.PrintString` "LEFT RADIUS" false true (struct :`R` 0.505208 :`A` 1.0) 5.0)
    (set `self.b_InItemRadZone` false)
    (`ActorComponent.Deactivate` (`self.Beeper`))))

(event `self.ReceiveTick`
  (params (DeltaSeconds :type "Float (single-precision)"))
  ;[1 1 1] MEMORY SOUND
  (if (`self.b_InItemRadZone`)
    (bind _asbp_main_character (cast `/Game/OctJam/Blueprints/Characters/BP_MainCharacter` (`GameplayStatics.GetPlayerCharacter` 0)))
    (bind _outhit (`KismetSystemLibrary.LineTraceSingle` (`SceneComponent.K2_GetComponentLocation` (`self.MemoryMesh`)) (+ (0.0 0.0 0.0) (* (`SceneComponent.K2_GetComponentLocation` (`Character.Mesh` _asbp_main_character)) 1.0)) "TraceTypeQuery1"))
    (bind (_bblockinghit _binitialoverlap _time _distance _location _impactpoint _normal _impactnormal _physmat _hitactor _hitcomponent _hitbonename _bonename _hititem _elementindex _faceindex _tracestart _traceend) (`GameplayStatics.BreakHitResult` _outhit))
    (bind _output_get (set `self.fvar_ItemCollisionPoint` (* (`KismetMathLibrary.GetPointDistanceToLine` _traceend _tracestart) -1.0)))
    (`ActorComponent.Activate` (`self.Beeper`) false)))

(fn `AdvanceNextLevel`
  (bind _returnvalue (`GameplayStatics.GetCurrentLevelName` true))
  (bind _returnvalue_2 (`|GetDataTableRow` "/Game/OctJam/Blueprints/DT_LevelProgression.DT_LevelProgression" (`KismetStringLibrary.Conv_StringToName` _returnvalue))
    (:`then`
      (`GameplayStatics.OpenLevel` (`KismetStringLibrary.Conv_StringToName` (`.NextLevelName_4_88270F95C3430190F88FBCBB9690428E` (break `/Game/OctJam/Blueprints/S_LevelData` _returnvalue_2)))))
    (:`RowNotFound`
      (`KismetSystemLibrary.PrintString` "ERROR: Issue finding next level" true true (struct :`G` 0.66 :`B` 1.0 :`A` 1.0) 10.0)
      (return) ; Continue game as normal
    )))

(fn `CollectItemWithDialogue`
  (params (OtherComp :type "PrimitiveComponent Object Reference") (Dialogue :type "DataTable Object Reference"))
  (bind _asbp_main_character (cast `/Game/OctJam/Blueprints/Characters/BP_MainCharacter` (`GameplayStatics.GetPlayerCharacter` 0)))
  (if (== (`Character.CapsuleComponent` _asbp_main_character) OtherComp)
    (`CharacterMovementComponent.SetMovementMode` (`Character.CharacterMovement` _asbp_main_character) "MOVE_None" 0)
    (`KismetSystemLibrary.PrintString` "Item Collected" true true (struct :`G` 0.66 :`B` 1.0 :`A` 1.0) 10.0)
    (`|ExecutionSequence`
      (:`then_0`
        (`self.K2_DestroyActor`))
      (:`then_1`
        (`self.CreateItemDialogue` Dialogue)))))

(fn `CreateItemDialogue`
  (params (ThisDT :type "DataTable Object Reference"))
  (`/Engine/EditorBlueprintResources/StandardMacros.IsValid` (`self.HUD_DialogueWidget`)
    (:`Is Valid`
      (`KismetSystemLibrary.PrintString` "UI VALID: Already Exists"))
    (:`Is Not Valid`
      (`KismetSystemLibrary.PrintString` "UI NOT VALID: Creating")
      (bind _returnvalue (`|CreateWidget` "/Game/OctJam/Blueprints/UI/HUD/HUD_Dialogue.HUD_Dialogue_C"))
      (bind _output_get (set `self.HUD_DialogueWidget` _returnvalue))))
  (`/Game/OctJam/Blueprints/UI/HUD/HUD_Dialogue.SwitchDT` _output_get ThisDT)
  (`UserWidget.AddToViewport` _output_get 0)
  (message `/Game/OctJam/Blueprints/BPI_ChangeLevel.SetLevelTrigger` _output_get (`self.b_isLevelTrigger`)))

(fn `PlayItemDescDialogue`
  (params (OtherComp :type "PrimitiveComponent Object Reference") (Dialogue :type "DataTable Object Reference"))
  (bind _asbp_main_character (cast `/Game/OctJam/Blueprints/Characters/BP_MainCharacter` (`GameplayStatics.GetPlayerCharacter` 0)))
  (`CharacterMovementComponent.SetMovementMode` (`Character.CharacterMovement` _asbp_main_character) "MOVE_None" 0)
  (if (== (`Character.CapsuleComponent` _asbp_main_character) OtherComp)
    (`KismetSystemLibrary.PrintString` "Playing Memory Description" true true (struct :`G` 0.66 :`B` 1.0 :`A` 1.0) 10.0)
    (`self.CreateItemDialogue` Dialogue)))

(fn `ShowExamineIndicator`
  (params (Component :type "PrimitiveComponent Object Reference") (Player :type "Actor Object Reference"))
  (if (`|EnumEquality` (`PrimitiveComponent.GetCollisionObjectType` Component) "ECC_GameTraceChannel2")
    (message `/Game/OctJam/Blueprints/BPI_Examine.ShowIndicator` Player)))

(fn `UpdateMemoryCounter`
  (bind _result (`/Engine/EditorBlueprintResources/StandardMacros.IncrementInt` (`self.i_itemIndex`))
    (:`  `
      (bind _output_get (set `self.i_itemIndex` _result))
      (switch `/Game/OctJam/Blueprints/UI/HUD/Enum/E_TTSMode` "NewEnumerator0"
        (:`NewEnumerator0`
          (switch `int` _output_get
            (:`1`
              (`KismetSystemLibrary.PrintString` "1 of 4 collected"))
            (:`2`
              (`KismetSystemLibrary.PrintString` "2 of 4 collected"))
            (:`3`
              (`KismetSystemLibrary.PrintString` "3 of 4 collected"))
            (:`4`
              (return) ; No need for TTS on 4/4 collected
            )))))))

(fn `UserConstructionScript`)