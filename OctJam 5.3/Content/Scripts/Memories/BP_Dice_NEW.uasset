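; Collectible dice memory item that builds on a parent Blueprint for its pickup behavior.
; On BeginPlay it sets the dice examine dialogue table as the current item description.
; Overlapping the CollectItem component passes the other component and the dice collision dialogue to CollectItemWithDialogue.
; An unconnected node for destroying its components remains in the graph and never runs.
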(event `self.ReceiveBeginPlay`
  (set `self.DT_CurrItemDescDT` "/Game/OctJam/Blueprints/UI/HUD/DataTables/Memories/Examine/DT_Dialogue_Examine_Dice.DT_Dialogue_Examine_Dice"))

(event `self.CollectItem.OnComponentBeginOverlap`
  (params (OverlappedComponent :type "PrimitiveComponent Object Reference") (OtherActor :type "Actor Object Reference") (OtherComp :type "PrimitiveComponent Object Reference") (OtherBodyIndex :type Integer) (bFromSweep :type Boolean) (SweepResult :type "HitResult Structure (by ref)"))
  (`self.CollectItemWithDialogue` OtherComp "/Game/OctJam/Blueprints/UI/HUD/DataTables/Memories/Collide/DT_Dialogue_Collide_Dice.DT_Dialogue_Collide_Dice"))

(fn `UserConstructionScript`
  (`parent.UserConstructionScript`))