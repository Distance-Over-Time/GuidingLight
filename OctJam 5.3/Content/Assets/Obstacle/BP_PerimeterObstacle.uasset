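; BP_PerimeterObstacle is an obstacle that plays directional audio when one of the player's four compass-point detection components enters its audio radius.
; On begin overlap it casts the player to BP_MainCharacter and matches the overlapping component to that character's North, East, West or South component.
; The matching audio component activates only if not already active.
; End overlap does nothing, as the logic that deactivates each sound is disconnected.
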(event `PlayAudioN`
  ;[1 1 1] North
  (`self.ActivateSoundAsNecessary` (`self.AudioN`)))

(event `PlayAudioE`
  ;[1 1 1] East
  (`self.ActivateSoundAsNecessary` (`self.AudioE`)))

(event `self.ObstacleRadius4Audio.OnComponentBeginOverlap`
  (params (OverlappedComponent :type "PrimitiveComponent Object Reference") (OtherActor :type "Actor Object Reference") (OtherComp :type "PrimitiveComponent Object Reference") (OtherBodyIndex :type Integer) (bFromSweep :type Boolean) (SweepResult :type "HitResult Structure (by ref)"))
  (`self.SetPlayerCast`
    (:`then`
      (`|ExecutionSequence`
        (:`then_0`
          ;[1 1 1] NORTH
          (if (== (`/Game/OctJam/Blueprints/Characters/BP_MainCharacter.ObstacleNORTH` (`self.PlayerCast`)) OtherComp)
            (`self.PlayAudioN`)))
        (:`then_1`
          ;[1 1 1] EAST
          (if (== (`/Game/OctJam/Blueprints/Characters/BP_MainCharacter.ObstacleEAST` (`self.PlayerCast`)) OtherComp)
            (`self.PlayAudioE`)))
        (:`then_2`
          ;[1 1 1] WEST
          (if (== (`/Game/OctJam/Blueprints/Characters/BP_MainCharacter.ObstacleWEST` (`self.PlayerCast`)) OtherComp)
            (`self.PlayAudioW`)))
        (:`then_3`
          ;[1 1 1] SOUTH
          (if (== (`/Game/OctJam/Blueprints/Characters/BP_MainCharacter.ObstacleSOUTH` (`self.PlayerCast`)) OtherComp)
            (`self.PlayAudioS`)))))
    (:`CastFailed`
      (`KismetSystemLibrary.PrintString` "can't cast to player cast var (obstacle start overlap)"))))

(event `PlayAudioW`
  ;[1 1 1] West
  (`self.ActivateSoundAsNecessary` (`self.AudioW`)))

(event `PlayAudioS`
  ;[1 1 1] South
  (`self.ActivateSoundAsNecessary` (`self.AudioS`)))

(event `self.ObstacleRadius4Audio.OnComponentEndOverlap`
  (params (OverlappedComponent :type "PrimitiveComponent Object Reference") (OtherActor :type "Actor Object Reference") (OtherComp :type "PrimitiveComponent Object Reference") (OtherBodyIndex :type Integer)))

(fn `UserConstructionScript`)