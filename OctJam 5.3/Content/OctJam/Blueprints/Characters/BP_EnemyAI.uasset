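; BP_EnemyAI is an enemy character that serves as an audio proximity hazard, warning the player as they get near.
; Inside TriggerRadius, Tick traces to the player, stores a negated distance and runs EnemyWarningSignal, though its pitch normalizes a constant rather than that distance.
; DangerSphere overlap retriggers DangerSound on short random delays, and capsule contact plays the death sound.
; SetUpPlayerCollision caches BP_MainCharacter and its capsule for overlap checks; no movement logic exists here.
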(event `self.ReceiveTick`
  (params (DeltaSeconds :type "Float (single-precision)"))
  (bind _enemywarningsignal (`self.EnemyWarningSignal`))
  (bind _obj_playercast (`self.obj_PlayerCast`))
  ;[0.6802 0.1356 0] Homing Signal
  (if (`self.b_inEnemyProximity`)
    (`/Engine/EditorBlueprintResources/StandardMacros.IsValid` _obj_playercast
      (:`Is Valid`
        (bind _outhit (`KismetSystemLibrary.LineTraceSingle` (`SceneComponent.K2_GetComponentLocation` (`self.CapsuleComponent`)) (+ (0.0 0.0 0.0) (* (`SceneComponent.K2_GetComponentLocation` (`Character.Mesh` _obj_playercast)) 1.0)) "TraceTypeQuery1"))
        (bind (_bblockinghit _binitialoverlap _time _distance _location _impactpoint _normal _impactnormal _physmat _hitactor _hitcomponent _hitbonename _bonename _hititem _elementindex _faceindex _tracestart _traceend) (`GameplayStatics.BreakHitResult` _outhit))
        (set `self.fvar_Enemy_Collision_Point` (* (`KismetMathLibrary.GetPointDistanceToLine` _traceend _tracestart) -1.0))
        (`ActorComponent.Activate` _enemywarningsignal false)
        (`AudioComponent.SetPitchMultiplier` _enemywarningsignal (+ (`KismetMathLibrary.NormalizeToRange` 0.0 -1646.0 -400.0) 1.0))))))

(event `self.TriggerRadius.OnComponentBeginOverlap`
  (params (OverlappedComponent :type "PrimitiveComponent Object Reference") (OtherActor :type "Actor Object Reference") (OtherComp :type "PrimitiveComponent Object Reference") (OtherBodyIndex :type Integer) (bFromSweep :type Boolean) (SweepResult :type "HitResult Structure (by ref)"))
  (bind _obj_playercollision (`self.obj_PlayerCollision`))
  ;[1 0.1544 0] What to do when player enters or exits the Enemy's radius
  (`/Engine/EditorBlueprintResources/StandardMacros.IsValid` _obj_playercollision :!label _label
    (:`Is Valid`
      (if (== OtherComp _obj_playercollision)
        (`KismetSystemLibrary.PrintString` "INSIDE RADIUS" false true (struct :`R` 0.041959 :`G` 0.505208 :`A` 1.0) 5.0)
        (set `self.b_inEnemyProximity` true)))
    (:`Is Not Valid`
      (`self.SetUpPlayerCollision`
        (:`output`
          (goto _label))))))

(event `self.ReceiveBeginPlay`
  (`self.SetUpPlayerCollision`))

(event `self.TriggerRadius.OnComponentEndOverlap`
  (params (OverlappedComponent :type "PrimitiveComponent Object Reference") (OtherActor :type "Actor Object Reference") (OtherComp :type "PrimitiveComponent Object Reference") (OtherBodyIndex :type Integer))
  ;[1 0.1544 0] What to do when player enters or exits the Enemy's radius
  (if (== (`self.obj_PlayerCollision`) OtherComp)
    (`KismetSystemLibrary.PrintString` "LEFT RADIUS" false true (struct :`R` 0.505208 :`A` 1.0) 5.0)
    (set `self.b_inEnemyProximity` false)
    (`ActorComponent.Deactivate` (`self.EnemyWarningSignal`))))

(event `self.CapsuleComponent.OnComponentBeginOverlap`
  (params (OverlappedComponent :type "PrimitiveComponent Object Reference") (OtherActor :type "Actor Object Reference") (OtherComp :type "PrimitiveComponent Object Reference") (OtherBodyIndex :type Integer) (bFromSweep :type Boolean) (SweepResult :type "HitResult Structure (by ref)"))
  (bind _obj_playercollision (`self.obj_PlayerCollision`))
  ;[1 0 0.008825] Death Sequence
  (`/Engine/EditorBlueprintResources/StandardMacros.IsValid` _obj_playercollision :!label _label_2
    (:`Is Valid`
      (if (== OtherComp _obj_playercollision)
        (`GameplayStatics.PlaySound2D` "/Game/Audio/SFX/PlayerAndEnemy/player_death_Cue.player_death_Cue" 1.0 1.0 0.0 null null)
        (`ActorComponent.Deactivate` (`self.DangerSound`))))
    (:`Is Not Valid`
      (`self.SetUpPlayerCollision`
        (:`output`
          (goto _label_2))))))

(event `self.DangerSphere.OnComponentBeginOverlap`
  (params (OverlappedComponent :type "PrimitiveComponent Object Reference") (OtherActor :type "Actor Object Reference") (OtherComp :type "PrimitiveComponent Object Reference") (OtherBodyIndex :type Integer) (bFromSweep :type Boolean) (SweepResult :type "HitResult Structure (by ref)"))
  (bind _dangersound (`self.DangerSound`))
  (bind _obj_playercollision (`self.obj_PlayerCollision`))
  ;[0.569 1 0.2776] Super Close to Enemy
  (`/Engine/EditorBlueprintResources/StandardMacros.IsValid` _obj_playercollision :!label _label_3
    (:`Is Valid`
      (if (== OtherComp _obj_playercollision)
        (set `self.b_EnemyClose` true)
        (if (`self.b_EnemyClose`) :!label _label_4
          (`ActorComponent.Activate` _dangersound false)
          (`KismetSystemLibrary.Delay` (`KismetMathLibrary.RandomFloatInRange` 0.0 0.05))
          (goto _label_4)
          (else
            (`ActorComponent.Deactivate` _dangersound)))))
    (:`Is Not Valid`
      (`self.SetUpPlayerCollision`
        (:`output`
          (goto _label_3))))))

(event `self.DangerSphere.OnComponentEndOverlap`
  (params (OverlappedComponent :type "PrimitiveComponent Object Reference") (OtherActor :type "Actor Object Reference") (OtherComp :type "PrimitiveComponent Object Reference") (OtherBodyIndex :type Integer))
  ;[0.569 1 0.2776] Super Close to Enemy
  (if (== (`self.obj_PlayerCollision`) OtherComp)
    (set `self.b_EnemyClose` false)))

(fn `UserConstructionScript`)