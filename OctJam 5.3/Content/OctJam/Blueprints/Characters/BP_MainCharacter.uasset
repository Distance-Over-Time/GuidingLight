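; Player character that examines environment objects through text-to-speech dialogue, pauses the game and respawns after death.
; DialogueTrigger overlaps on custom collision channels enable examining and call GetObjMessage on the object, while SendDT stores the current DataTable.
; Examine feeds that table to a reused HUD widget and disables movement.
; Destruction triggers a black-screen fade, GameMode respawn and sound, plus hazard-restart dialogue in level2_patch.
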(event `self.ReceiveDestroyed`
  ;[1 0.07081 0.1305] DEATH DIALOGUE
  (`self.DeathSequence`))

(event `/Game/OctJam/Blueprints/BPI_EnvInteraction.SendDT`
  (params (`Data Table` :type "DataTable Object Reference"))
  ;[1 1 1] ENVIRONMENT TTS INTERACTION
  (set `self.DT_CurrEnv` `Data Table`))

(event `self.DialogueTrigger.OnComponentBeginOverlap`
  (params (OverlappedComponent :type "PrimitiveComponent Object Reference") (OtherActor :type "Actor Object Reference") (OtherComp :type "PrimitiveComponent Object Reference") (OtherBodyIndex :type Integer) (bFromSweep :type Boolean) (SweepResult :type "HitResult Structure (by ref)"))
  (bind _returnvalue (`PrimitiveComponent.GetCollisionObjectType` OtherComp))
  ;[1 1 1] ENVIRONMENT TTS INTERACTION
  (switch `ECollisionChannel` _returnvalue
    (:`ECC_GameTraceChannel1`
      _)
    (:`ECC_GameTraceChannel2`
      _))
  (`self.CheckIfExaminable` _returnvalue true)
  (message `/Game/OctJam/Blueprints/BPI_EnvInteraction.GetObj` OtherActor))

(event `InputAction|OpenMenu`
  (params (Key :type "Key Structure"))
  ;[1 0.8096 0.3512] PAUSE MENU
  (:`Pressed`
    (`self.PauseGame`)))

(event `self.DialogueTrigger.OnComponentEndOverlap`
  (params (OverlappedComponent :type "PrimitiveComponent Object Reference") (OtherActor :type "Actor Object Reference") (OtherComp :type "PrimitiveComponent Object Reference") (OtherBodyIndex :type Integer))
  ;[1 1 1] ENVIRONMENT TTS INTERACTION
  (set `self.b_CanExamine` false)
  (`self.IndicateExamine` false))

(event `self.ObstacleStopper.OnComponentBeginOverlap`
  (params (OverlappedComponent :type "PrimitiveComponent Object Reference") (OtherActor :type "Actor Object Reference") (OtherComp :type "PrimitiveComponent Object Reference") (OtherBodyIndex :type Integer) (bFromSweep :type Boolean) (SweepResult :type "HitResult Structure (by ref)"))
  ;[1 0 0.4136] Obstacle Stopper/Indicator
  (if (`self.ActorHasTag` OtherActor "Wall")
    (`GameplayStatics.PlaySound2D` "/Game/Audio/SFX/Accessibility/wall_hit.wall_hit" 1.0 1.0 0.0 null null)))

(event `InputAction|Examine`
  (params (Key :type "Key Structure"))
  ;[1 1 1] ENVIRONMENT TTS INTERACTION
  (:`Pressed`
    (if (`self.b_CanExamine`)
      (`self.ExamineEnv` (`self.DT_CurrEnv`))
      (set `self.b_CanExamine` false)
      (else
        (`KismetSystemLibrary.PrintString` "Can't examine")))))

(event `/Game/OctJam/Blueprints/BPI_Examine.ShowIndicator`
  ;[1 1 1] ENVIRONMENT TTS INTERACTION
  (`self.IndicateExamine` true))

(event `/Game/OctJam/Blueprints/BPI_Examine.RemoveIndicator`
  ;[1 1 1] ENVIRONMENT TTS INTERACTION
  (`self.IndicateExamine` false))

(fn `CheckIfExaminable`
  (params (`TTS Collision Type` :type "ECollisionChannel Enum" :default "ECC_WorldStatic") (Toggle :type Boolean))
  (if (or (`|EnumEquality` `TTS Collision Type` "ECC_GameTraceChannel2") (`|EnumEquality` `TTS Collision Type` "ECC_GameTraceChannel1"))
    (set `self.b_CanExamine` Toggle)))

(fn `ExamineEnv`
  (params (`Env DT` :type "DataTable Object Reference"))
  (`/Engine/EditorBlueprintResources/StandardMacros.IsValid` (`self.HUD_Player`)
    (:`Is Valid`
      (`KismetSystemLibrary.PrintString` "UI VALID: Already Exists"))
    (:`Is Not Valid`
      (`KismetSystemLibrary.PrintString` "UI NOT VALID: Creating")
      (bind _returnvalue (`|CreateWidget` "/Game/OctJam/Blueprints/UI/HUD/HUD_Dialogue.HUD_Dialogue_C"))
      (bind _output_get (set `self.HUD_Player` _returnvalue))))
  (`/Game/OctJam/Blueprints/UI/HUD/HUD_Dialogue.SwitchDT` _output_get `Env DT`)
  (`UserWidget.AddToViewport` _output_get 0)
  (`CharacterMovementComponent.SetMovementMode` (`self.CharacterMovement`) "MOVE_None" 0)
  (`self.IndicateExamine` false))

(fn `IndicateExamine`
  (params (`Show Indicator` :type Boolean))
  (bind _aud_examine (`self.AUD_Examine`))
  (`SceneComponent.SetVisibility` (`self.ExamineIcon`) `Show Indicator` false)
  (if `Show Indicator`
    (`AudioComponent.Play` _aud_examine 0.0)
    (else
      (`AudioComponent.Stop` _aud_examine))))

(fn `PauseGame`
  (bind _returnvalue (`GameplayStatics.GetPlayerController` 0))
  (`GameplayStatics.SetGamePaused` true)
  (bind _returnvalue_2 (`|CreateWidget` "/Game/OctJam/Blueprints/UI/WBP_PauseMenu.WBP_PauseMenu_C" _returnvalue))
  (`WidgetBlueprintLibrary.SetInputMode_GameAndUIEx` _returnvalue _returnvalue_2)
  (`UserWidget.AddToViewport` _returnvalue_2 0))

(fn `ResumeGame`
  (bind _hud_player (`self.HUD_Player`))
  (`GameplayStatics.SetGamePaused` false)
  (`/Engine/EditorBlueprintResources/StandardMacros.IsValid` _hud_player
    (:`Is Valid`
      (`Widget.RemoveFromParent` _hud_player)
      (`WidgetBlueprintLibrary.SetInputMode_GameOnly` (`GameplayStatics.GetPlayerController` 0) true)
      (message `/Game/OctJam/Blueprints/BPI_PauseTTS.ResumeTTS` _hud_player))))

(fn `UserConstructionScript`)